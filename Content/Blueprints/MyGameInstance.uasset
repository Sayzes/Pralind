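; Game instance that creates a multiplayer session to host a lobby.
; The Createlobby event stores the server name, map, slots, mode and LAN choice, then passes them to an Advanced Sessions node as connection options and custom session properties.
; On success it opens the hardcoded Map1 as a listen server, regardless of the chosen map, and failure is not handled.
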(event Custom|Createlobby
  (params (Servername :type String) (Servermap :type String) (Serverslot :type Integer) (Servermode :type String) (Servermethod_LAN? :type Boolean))
  (Variables|Default|SetServername Servername)
  (Variables|Default|SetServermap Servermap)
  (Variables|Default|SetServerslot Serverslot)
  (Variables|Default|SetServermode Servermode)
  (Variables|Default|SetServermethod_LAN? Servermethod_LAN?)
  (|AdvancedSession (Utilities|Array|MakeArray (Class|AdvancedSessionsLibrary|MakeLiteralSessionPropertyString "NAME" (Variables|Default|GetServername)) (Class|AdvancedSessionsLibrary|MakeLiteralSessionPropertyString "MAP" (Variables|Default|GetServermap)) (Class|AdvancedSessionsLibrary|MakeLiteralSessionPropertyString "MODE" (Variables|Default|GetServermode)) (Class|AdvancedSessionsLibrary|MakeLiteralSessionPropertyBool "LAN" (Variables|Default|GetServermethod_LAN?))) (Game|GetPlayerController 0) 100 (Variables|Default|GetServerslot) (Variables|Default|GetServermethod_LAN?) true false true true false false false true
    (:OnSuccess
      (Game|OpenLevel(byName) "Map1" true "listen"))))